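; BP_Dirt is a dirt decal that fades as a motion-controller-held BP_Brush scrubs it.
; Box overlaps track brush contact and cache the holding controller, whose speed CleanDirt checks every Tick.
; Fast strokes lower a dynamic material's opacity by a fixed per-frame step and trigger Niagara and brush sound.
; Sound stops on overlap end or after a tick-counted slow period, which also re-arms the effect.
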(event OnComponentBeginOverlap(Box)
  (params (OverlappedComponent :type Primitive%20Component%20Object%20Reference) (OtherActor :type Actor%20Object%20Reference) (OtherComp :type Primitive%20Component%20Object%20Reference) (OtherBodyIndex :type Integer) (bFromSweep :type Boolean) (SweepResult :type Hit%20Result%20Structure%20%28by%20ref%29))
  (bind _asbp_brush (Utilities|Casting|CastToBP_Brush OtherActor)
    (:then
      (Variables|Default|SetIsBrushStartedCollision true)
      (bind _returnvalue (Class|MFKGrabComponent|GetHoldingMotionController (Actor|GetComponentbyClass _asbp_brush "/Script/MFKHands.MFKGrabComponent")))
      (Variables|Default|SetBrushMotionController _returnvalue))
    (:CastFailed
      (Development|PrintString "fail no brush"))))

(event OnComponentEndOverlap(Box)
  (params (OverlappedComponent :type Primitive%20Component%20Object%20Reference) (OtherActor :type Actor%20Object%20Reference) (OtherComp :type Primitive%20Component%20Object%20Reference) (OtherBodyIndex :type Integer))
  (bind _brushsound (Variables|Default|GetBrushSound))
  (Utilities|Casting|CastToBP_Brush OtherActor)
  (Variables|Default|SetIsBrushStartedCollision false)
  (Utilities|IsValid _brushsound
    (:Is%20Valid
      (Audio|Components|Audio|Stop _brushsound)
      (Variables|Default|SetIsSoundPlaying false))))

(event EventBeginPlay
  (bind _returnvalue (Rendering|Material|CreateDynamicMaterialInstance "/Game/_Game_/Models/Horse/Decal/M_dirtDecal.M_dirtDecal" "None" "None" :!class /Script/Engine.KismetMaterialLibrary))
  (bind _output_get (Variables|Default|SetDirtMaterialInstance _returnvalue))
  (Rendering|Components|Decal|SetDecalMaterial (Variables|Default|GetDecal) _output_get))

(event Collision|EventActorBeginOverlap
  (params (OtherActor :type Actor%20Object%20Reference)))

(event EventTick
  (params (DeltaSeconds :type Float%20%28single-precision%29))
  (CallFunction|CleanDirt))

(fn ConstructionScript)

(fn CleanDirt
  (bind _brushmotioncontroller (Variables|Default|GetBrushMotionController))
  (bind _dirtmaterialinstance (Variables|Default|GetDirtMaterialInstance))
  (bind _outlinearvelocity (Class|MotionControllerComponent|GetLinearVelocity _brushmotioncontroller))
  (bind _returnvalue (Math|Vector|VectorLength _outlinearvelocity))
  (if (Variables|Default|GetIsBrushStartedCollision)
    (Development|PrintString (Utilities|String|ToString(Float) _returnvalue) true true "(R=1.000000,G=0.046124,B=0.000000,A=1.000000)" 0.1)
    (if (>= _returnvalue 35.0)
      (bind _returnvalue_2 (Rendering|Material|GetScalarParameterValue _dirtmaterialinstance "DirtOpacity" :!class /Script/Engine.MaterialInstanceDynamic))
      (Rendering|Material|SetScalarParameterValue _dirtmaterialinstance "DirtOpacity" (- _returnvalue_2 0.005) :!class /Script/Engine.MaterialInstanceDynamic)
      (Variables|Default|SetafkTime 0.0)
      (Development|PrintString "afk time reseted" true true "(R=1.000000,G=0.885502,B=0.000000,A=1.000000)")
      (Utilities|FlowControl|Sequence
        (:then_0
          (if (not (Variables|Default|GetIsNiagaraActive))
            (bind _returnvalue_3 (Niagara|SpawnSystematLocation "/Game/_Game_/vfx/NiagaStarterPack/Realistic_Starter_VFX_Pack_Niagara/Niagara/Smoke_and_Steam/NS_HorseTOz.NS_HorseTOz" (Transformation|GetWorldLocation (Variables|Default|GetDefaultSceneRoot)) "0, 0, 0" "1.000000,1.000000,1.000000" true true "AutoRelease"))
            (Variables|Default|SetNiagara _returnvalue_3)
            (Variables|Default|SetIsNiagaraActive true)))
        (:then_1
          (if (not (Variables|Default|GetIsSoundPlaying))
            (bind _returnvalue_4 (Audio|SpawnSoundAttached "/Game/_Game_/Sounds/BrushSFX/brush_Cue.brush_Cue" (Variables|Default|GetDefaultSceneRoot) "None" "0, 0, 0" "0, 0, 0" "KeepRelativeOffset" false 1.0 1.0 0.0 0 0))
            (Variables|Default|SetBrushSound _returnvalue_4)
            (Audio|Components|Audio|Play (Variables|Default|GetBrushSound) 0.0)
            (Variables|Default|SetIsSoundPlaying true)
            (Development|PrintString "BAŞLADIIII"))))
      (else
        (Development|PrintString "timer STartedddd" false true "(R=0.000000,G=0.430671,B=1.000000,A=1.000000)")
        (if (Variables|Default|GetIsSoundPlaying)
          (bind _output_get (Variables|Default|SetafkTime (+ (Variables|Default|GetafkTime) 0.4)))
          (Development|PrintString (Utilities|String|ToString(Float) _output_get))
          (if (> (Variables|Default|GetafkTime) 1e+01)
            (Audio|Components|Audio|Stop (Variables|Default|GetBrushSound))
            (Variables|Default|SetIsSoundPlaying false)
            (Development|PrintString "soun durduuuu" true true "(R=1.000000,G=0.038842,B=0.000000,A=1.000000)")
            (if (Variables|Default|GetIsNiagaraActive)
              (Variables|Default|SetIsNiagaraActive false)))
          (else
            (Development|PrintString "is sound palyinggg nooooooooooooooooooooooooooooo" true true "(R=1.000000,G=0.000000,B=0.048026,A=1.000000)")))))))

(fn DisableSound
  (Development|PrintString "disable a girdin ama sound oynamıyor kiii")
  (if (Variables|Default|GetIsSoundPlaying)
    (Development|PrintString "stopppppp sounddddd")
    (Audio|Components|Audio|Stop (Variables|Default|GetBrushSound))
    (Variables|Default|SetIsSoundPlaying false)))