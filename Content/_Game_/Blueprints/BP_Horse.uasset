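; BP_Horse is a horse actor that snorts periodically and eats food held by an MFK grab hand.
; A looping timer, its interval randomized once at BeginPlay, plays the snort sound.
; Box overlap with a "food"-tagged actor resets the holding hand's grab pose to Free, destroys the food, and plays eating audio and montage.
; A flag blocks repeat eating until montage completion, but stays set if the hand AnimInstance cast fails.
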(event OnComponentBeginOverlap(Box)
  (params (OverlappedComponent :type Primitive%20Component%20Object%20Reference) (OtherActor :type Actor%20Object%20Reference) (OtherComp :type Primitive%20Component%20Object%20Reference) (OtherBodyIndex :type Integer) (bFromSweep :type Boolean) (SweepResult :type Hit%20Result%20Structure%20%28by%20ref%29))
  (if (Variables|Default|GetIsAlreadyEating)
    (Development|PrintString "already eating ")
    (elif (Actor|ActorHasTag OtherActor "food")
      (Variables|Default|SetIsAlreadyEating true)
      (bind _returnvalue (Class|MFKGrabComponent|GetHoldingSkeletalMeshComponent (Actor|GetComponentbyClass OtherActor "/Script/MFKHands.MFKGrabComponent")))
      (bind _asmfkhand_anim_instance (Utilities|Casting|CastToMFKHandAnimInstance (Components|SkeletalMesh|GetAnimInstance _returnvalue))
        (:then
          (Variables|/Script/MFKHands.MFKHandAnimInstance|SetCurrentGrabType _asmfkhand_anim_instance "Free")
          (Actor|DestroyActor OtherActor)
          (Audio|PlaySoundatLocation "/Game/_Game_/Sounds/HorseSFX/HorseEating_1_Cue.HorseEating_1_Cue" (Transformation|GetWorldLocation (Variables|Default|GetBox)) "0, 0, 0" 1.0 1.0 0.0 0 0 0 0)
          (Animation|Montage|PlayMontage (Variables|Default|GetSkeletalMesh) "/Game/_Game_/Models/Horse/alprnHorse/anims/Horse_Eat_Motion_Montage.Horse_Eat_Motion_Montage"
            (:OnCompleted
              (Variables|Default|SetIsAlreadyEating false))))
        (:CastFailed
          (Development|PrintString "mfkhandanim instance a castt fail oldu" true true "(R=1.000000,G=0.102204,B=0.000000,A=1.000000)" 1e+01)))
      (else
        (Development|PrintString "no food")))))

(event Custom|horsesnort
  (Audio|PlaySoundatLocation "/Game/_Game_/Sounds/HorseSFX/HorseSnort_Cue.HorseSnort_Cue" (Transformation|GetWorldLocation (Variables|Default|GetBox)) "0, 0, 0" 1.0 1.0 0.0 0 0 0 0))

(event EventBeginPlay
  (Development|PrintString "Hello")
  (Development|PrintString "saniye sonra")
  (Utilities|Time|SetTimerbyEvent (delegate Custom|horsesnort) (Math|Random|RandomFloatinRange 5.0 15.0) true))

(event Collision|EventActorBeginOverlap
  (params (OtherActor :type Actor%20Object%20Reference)))

(event EventTick
  (params (DeltaSeconds :type Float%20%28single-precision%29)))

(fn ConstructionScript)