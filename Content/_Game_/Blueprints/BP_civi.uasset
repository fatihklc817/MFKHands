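; BP_civi is a nail ("çivi") that the player hammers down with a motion-controller-held BP_Hammer1.
; When the hammer's "trigger" component overlaps the Box, the controller's clamped linear velocity sets how far the actor moves along local Z, capped by DistanceLeftToBeDone.
; Each hit plays a sound, starts a short timer-based debounce, sets holding flags on the Farmer and Horse AnimBlueprints and plays their hit montages.
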(event OnComponentBeginOverlap(Box)
  (params (OverlappedComponent :type Primitive%20Component%20Object%20Reference) (OtherActor :type Actor%20Object%20Reference) (OtherComp :type Primitive%20Component%20Object%20Reference) (OtherBodyIndex :type Integer) (bFromSweep :type Boolean) (SweepResult :type Hit%20Result%20Structure%20%28by%20ref%29))
  (if (> (Variables|Default|GetdistanceLeftToBeDone) 0.0)
    (if (not (Variables|Default|GetIsHitted))
      (bind _asbp_hammer_1 (Utilities|Casting|CastToBP_Hammer1 OtherActor)
        (:then
          (if (Components|ComponentHasTag OtherComp "trigger")
            (bind _returnvalue (Class|MFKGrabComponent|GetHoldingMotionController (Actor|GetComponentbyClass _asbp_hammer_1 "/Script/MFKHands.MFKGrabComponent")))
            (Development|PrintString (Utilities|String|Append "velocity lentgh : 
" (Utilities|String|ToString(Float) (Math|Vector|VectorLength (.OutLinearVelocity (Class|MotionControllerComponent|GetLinearVelocity _returnvalue))))) true true "(R=1.000000,G=0.228745,B=0.440543,A=1.000000)")
            (Development|PrintString (Utilities|String|Append "z - lenth is :  " (Utilities|String|ToString(Float) (/ 2.0 (/ 2e+02 (Math|Float|Clamp(Float) (Math|Vector|VectorLength (.OutLinearVelocity (Class|MotionControllerComponent|GetLinearVelocity _returnvalue))) 0.0 2e+02))))))
            (if (>= (/ 2.0 (/ 2e+02 (Math|Float|Clamp(Float) (Math|Vector|VectorLength (.OutLinearVelocity (Class|MotionControllerComponent|GetLinearVelocity _returnvalue))) 0.0 2e+02))) (Variables|Default|GetdistanceLeftToBeDone))
              (Variables|Default|SetaddingFloat (* (Variables|Default|GetdistanceLeftToBeDone) -1.0))
              (else
                (Variables|Default|SetaddingFloat (* (/ 2.0 (/ 2e+02 (Math|Float|Clamp(Float) (Math|Vector|VectorLength (.OutLinearVelocity (Class|MotionControllerComponent|GetLinearVelocity _returnvalue))) 0.0 2e+02))) -1.0))))
            (Transformation|AddActorLocalOffset (Math|Vector|MakeVector 0.0 0.0 (Variables|Default|GetaddingFloat)) false false)
            (Variables|Default|SetdistanceLeftToBeDone (+ (Variables|Default|GetdistanceLeftToBeDone) (Variables|Default|GetaddingFloat)))
            (Audio|PlaySoundatLocation "/Game/_Game_/Sounds/SC_LastHamemr01_Cue.SC_LastHamemr01_Cue" (Transformation|GetActorLocation) "0, 0, 0" 1.0 1.0 0.0 0 0 0 0)
            (Variables|Default|SetIsHitted true)
            (Utilities|Time|SetTimerbyEvent (delegate Custom|setIsHittedFalseAgain) 0.25)
            ;[1 1 1] hit
            (bind _asfarmer_t_anim_blueprint (Utilities|Casting|CastToFarmer_T_AnimBlueprint (Components|SkeletalMesh|GetAnimInstance (Variables|/Game/_Game_/Blueprints/BP_Farmer.BP_Farmer_C|GetSkeletalMesh (Variables|Default|Getfarmer))))
              (:then
                (Variables|/Game/_Game_/Models/Farmer/Farmer_T_AnimBlueprint.Farmer_T_AnimBlueprint_C|SetIsHolding _asfarmer_t_anim_blueprint true)
                (bind _ashorse_t_anim_blueprint (Utilities|Casting|CastToHorse_T_AnimBlueprint (Components|SkeletalMesh|GetAnimInstance (Variables|/Game/_Game_/Blueprints/BP_Horse.BP_Horse_C|GetSkeletalMesh (Variables|Default|Gethorse)))))
                (Variables|/Game/_Game_/Models/Horse/alprnHorse/Horse_T_AnimBlueprint.Horse_T_AnimBlueprint_C|SetIsLoopHolding _ashorse_t_anim_blueprint true)
                (Animation|Montage|PlayMontage (Variables|/Game/_Game_/Blueprints/BP_Horse.BP_Horse_C|GetSkeletalMesh (Variables|Default|Gethorse)) "/Game/_Game_/Models/Horse/alprnHorse/anims/Horse_Hit_Motion_Montage.Horse_Hit_Motion_Montage"
                  (:then
                    (Animation|Montage|PlayMontage (Variables|/Game/_Game_/Blueprints/BP_Farmer.BP_Farmer_C|GetSkeletalMesh (Variables|Default|Getfarmer)) "/Game/_Game_/Models/Farmer/anims/Farmer_Hit_Motion_Montage.Farmer_Hit_Motion_Montage"))))
              (:CastFailed
                (Development|PrintString "fail")))))
        (:CastFailed
          (Development|PrintString "fail no hammer"))))
    (else
      (Development|PrintString "çivi oturduuuuu" true true "(R=0.192751,G=0.000000,B=1.000000,A=1.000000)"))))

(event Custom|setIsHittedFalseAgain
  (Variables|Default|SetIsHitted false))

(event EventBeginPlay)

(event Collision|EventActorBeginOverlap
  (params (OtherActor :type Actor%20Object%20Reference)))

(event EventTick
  (params (DeltaSeconds :type Float%20%28single-precision%29)))

(fn ConstructionScript)